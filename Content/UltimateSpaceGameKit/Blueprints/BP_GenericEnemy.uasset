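; Generic enemy spaceship that flies around the player, fires inaccurate projectiles within an attack cone, and explodes in stages on death.
; Tick steers floating-pawn movement through randomly chosen patrol, circling or attack-run behaviors, with sphere-trace avoidance.
; A spring arm's length offsets the lead-targeting indicator by velocity and distance.
; Damage updates marker and cockpit-scanner feedback, while a distance check disables ticking when the player is far away.
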(event Custom|ExecuteBehaviour
  (bind _sphere (Variables|Default|GetSphere))
  ;[0 0 0] Execute behaviors
  (if (Variables|Default|GetIsAlive)
    (switch Utilities|FlowControl|Switch|SwitchonE_EnemyBehaviour (Variables|Default|GetBehaviour)
      (:NewEnumerator0
        (CallFunction|CircleinFrontOfPlayer))
      (:NewEnumerator1
        (CallFunction|FindDistanceandAttack))
      (:NewEnumerator2
        (CallFunction|CircleAroundPoint))
      (:NewEnumerator3
        (CallFunction|SimplePatrol)))
    (else
      (Class|PawnMovementComponent|AddInputVector (Variables|Default|GetFloatingPawnMovement) (+ (* (Math|Vector|GetForwardVector _sphere) 1e+03) (* (Math|Vector|GetRightVector _sphere) 1.0)) true)
      (Transformation|AddWorldRotation (Variables|Default|GetSphere) "1.000000, 0,3.000000" false false))))

(event Custom|CircleAroundPoint
  ;[0 0 0] Behaviours
  (bind _output_get (Variables|Default|SetInputVector (+ (Math|Interpolation|VInterpTo (Variables|Default|GetInputVector) (* (Math|Vector|GetForwardVector (Math|Rotator|FindLookatRotation (Transformation|GetActorLocation) (Transformation|GetActorLocation (Variables|Default|GetPlayerRef)))) 1e+03) (Utilities|Time|GetWorldDeltaSeconds) 1.0) (* (Math|Vector|GetForwardVector (Variables|Default|GetSphere)) 1e+01))))
  (Class|PawnMovementComponent|AddInputVector (Variables|Default|GetFloatingPawnMovement) _output_get false)
  (Variables|/Script/Engine.FloatingPawnMovement|SetMaxSpeed (Variables|Default|GetFloatingPawnMovement) 1.5e+04))

(event Custom|FindDistanceAndAttack
  (bind _self self)
  (bind _playerref (Variables|Default|GetPlayerRef))
  (bind _playerref_2 (Variables|Default|GetPlayerRef))
  (bind _playerref_3 (Variables|Default|GetPlayerRef))
  (bind _returnvalue (Transformation|GetDistanceTo _playerref _self))
  ;[0 0 0] Behaviours
  (if (Variables|Default|GetAttackFromDistance)
    (bind _output_get (Variables|Default|SetInputVector (Math|Interpolation|VInterpTo (Variables|Default|GetInputVector) (* (Math|Vector|GetForwardVector (Math|Rotator|FindLookatRotation (Transformation|GetActorLocation) (+ (Transformation|GetActorLocation _playerref_2) (* (Transformation|GetActorForwardVector _playerref_2) 3e+03) "0,0,-500.000000"))) 1e+04) (Utilities|Time|GetWorldDeltaSeconds) (Math|Float|MapRangeClamped (Transformation|GetDistanceTo (Variables|Default|GetPlayerRef)) 2e+03 1.5e+05 0.5 0.05))))
    (Class|PawnMovementComponent|AddInputVector (Variables|Default|GetFloatingPawnMovement) _output_get false)
    (Variables|/Script/Engine.FloatingPawnMovement|SetMaxSpeed (Variables|Default|GetFloatingPawnMovement) (Math|Float|MapRangeClamped _returnvalue 5e+03 9.5e+04 1e+04 4e+04))
    (if (< _returnvalue 1e+04)
      (Variables|Default|SetAttackFromDistance false))
    (else
      (bind _output_get_2 (Variables|Default|SetInputVector (Math|Interpolation|VInterpTo (Variables|Default|GetInputVector) (* (Math|Vector|GetForwardVector (Math|Rotator|FindLookatRotation (Transformation|GetActorLocation) (+ (Transformation|GetActorLocation _playerref_3) (* (Transformation|GetActorForwardVector _playerref_3) 2e+05) ""))) 5e+02) (Utilities|Time|GetWorldDeltaSeconds) 0.6)))
      (Class|PawnMovementComponent|AddInputVector (Variables|Default|GetFloatingPawnMovement) _output_get_2 false)
      (Variables|/Script/Engine.FloatingPawnMovement|SetMaxSpeed (Variables|Default|GetFloatingPawnMovement) 3e+04)
      (if (> (Transformation|GetDistanceTo (Variables|Default|GetPlayerRef) self) 1.2e+05)
        (Variables|Default|SetAttackFromDistance true)))))

(event Custom|Fire
  (bind _weaponl (Variables|Default|GetWeaponL))
  (bind _accuracyvariation (Variables|Default|GetAccuracyVariation))
  (bind _accuracyvariation_2 (Variables|Default|GetAccuracyVariation))
  (bind _accuracyvariation_3 (Variables|Default|GetAccuracyVariation))
  (bind _weaponl_2 (Variables|Default|GetWeaponL))
  (bind _returnvalue (Transformation|GetWorldTransform _weaponl))
  ;[0 0 0] Firing
  (Utilities|IsValid (Variables|Default|GetPlayerRef)
    (:Is%20Valid
      _)
    (:Is%20Not%20Valid
      (bind _asbp_player_ship (Utilities|Casting|CastToBP_PlayerShipdasda (Game|Player|GetPlayerPawn 0)))
      (Variables|Default|SetPlayerRef _asbp_player_ship)))
  (bind _iswithinangle (CallFunction|IsTargetWithinAngle (Variables|Default|GetPlayerRef) (Variables|Default|GetAttackConeAngleMax)))
  (if (Math|Boolean|ANDBoolean _iswithinangle (Math|Random|RandomBoolwithWeight (Variables|Default|GetChanceOfFiring)) (Variables|Default|GetIsAlive))
    (Transformation|SetWorldRotation _weaponl_2 (Math|Rotator|FindLookatRotation (Transformation|GetWorldLocation _weaponl_2) (+ (Transformation|GetActorLocation (Variables|Default|GetPlayerRef)) (Math|Vector|MakeVector (Math|Random|RandomFloatinRange (* _accuracyvariation_2 -1.0) _accuracyvariation_2) (Math|Random|RandomFloatinRange (* _accuracyvariation_3 -1.0) _accuracyvariation_3) (Math|Random|RandomFloatinRange (* _accuracyvariation -1.0) _accuracyvariation)))) false false)
    (bind _returnvalue_2 (Game|SpawnActorfromClass (Variables|Default|GetEnemyProjectile) (Math|Transform|MakeTransform (.location _returnvalue) (.rotation _returnvalue) "1.000000,1.000000,1.000000") "Undefined" "SelectDefaultAtRuntime" 0 0))
    (bind _asbp_laser_projectile (Utilities|Casting|CastToBP_LaserProjectile _returnvalue_2))
    (Variables|/Game/UltimateSpaceGameKit/Blueprints/BP_LaserProjectile.BP_LaserProjectile_C|SetSourceActor%28Weapon%29 _asbp_laser_projectile self)
    (Utilities|FlowControl|DoOnce false
      (:Completed
        (CallFunction|ChooseBehavior)))))

(event Custom|CheckForTarget
  ;[0 0 0] Firing
  (Utilities|Time|SetTimerbyEvent (EventDispatchers|CreateEvent :!event Custom|Fire) 0.16 true))

(event Custom|CircleInFrontOfPlayer
  (bind _playerref (Variables|Default|GetPlayerRef))
  ;[0 0 0] Behaviours
  (bind _output_get (Variables|Default|SetInputVector (Math|Interpolation|VInterpTo (Variables|Default|GetInputVector) (* (Math|Vector|GetForwardVector (Math|Rotator|FindLookatRotation (Transformation|GetActorLocation) (+ (Transformation|GetActorLocation _playerref) (* (Transformation|GetActorForwardVector _playerref) 3e+04) "0,0,1000.000000"))) 5e+04) (Utilities|Time|GetWorldDeltaSeconds) (Math|Float|MapRangeClamped (Transformation|GetDistanceTo (Variables|Default|GetPlayerRef)) 2.5e+04 5e+04 0.01 0.3))))
  (Class|PawnMovementComponent|AddInputVector (Variables|Default|GetFloatingPawnMovement) _output_get false)
  (Variables|/Script/Engine.FloatingPawnMovement|SetMaxSpeed (Variables|Default|GetFloatingPawnMovement) (Math|Float|MapRangeClamped (Transformation|GetDistanceTo (Variables|Default|GetPlayerRef)) 2.5e+04 8e+04 1.5e+04 4e+04)))

(event Custom|SimplePatrol
  (bind _sphere (Variables|Default|GetSphere))
  ;[0 0 0] Behaviours
  (bind _output_get (Variables|Default|SetInputVector (+ (* (Math|Vector|GetRightVector _sphere) 0.02) (* (Math|Vector|GetForwardVector _sphere) 1.0))))
  (Class|PawnMovementComponent|AddInputVector (Variables|Default|GetFloatingPawnMovement) _output_get false)
  (Variables|/Script/Engine.FloatingPawnMovement|SetMaxSpeed (Variables|Default|GetFloatingPawnMovement) 4e+03)
  (if (< (Transformation|GetDistanceTo (Variables|Default|GetPlayerRef)) 1e+05)
    (Utilities|FlowControl|DoOnce false
      (:Completed
        (CallFunction|ChooseBehavior)))))

(event Custom|ChooseBehavior
  ;[1 1 1] initialize
  (Variables|Default|SetBehaviour (Utilities|Enum|ByteToEnumE_EnemyBehaviour (Math|Conversions|ToByte(Integer) (Math|Random|RandomIntegerinRange 0 3))))
  (Utilities|Time|SetTimerbyEvent (EventDispatchers|CreateEvent :!event Custom|ChooseBehavior) (Math|Random|RandomFloatinRange 5.0 8.0)))

(event Custom|DistanceRelevancy
  (bind _returnvalue (Game|Player|GetPlayerPawn 0))
  ;[1 1 1] Disable actors ticking if too far from the player (if player travels to a different sector)
  (Utilities|IsValid _returnvalue
    (:Is%20Valid
      (if (> (Transformation|GetDistanceTo _returnvalue) 3e+05)
        (Actor|Tick|SetActorTickEnabled false)
        (else
          (Actor|Tick|SetActorTickEnabled true))))))

(event Custom|PlayerHitsTarget_Feedback
  (bind _widget_markerandhealth (Variables|Default|GetWidget_MarkerAndHealth))
  ;[1 1 1] Display UI element inside ship
  (Utilities|FlowControl|Sequence
    (:then_0
      (Utilities|IsValid _widget_markerandhealth
        (:Is%20Valid
          (bind _aswbp_enemy_marker_and_health (Utilities|Casting|CastToWBP_EnemyMarkerAndHealth (UserInterface|GetWidget _widget_markerandhealth)))
          (Default|PlayMarkerEnemyHitAnim _aswbp_enemy_marker_and_health)
          (Progress|SetPercent (Variables|/Game/UltimateSpaceGameKit/UI/WBP_EnemyMarkerAndHealth.WBP_EnemyMarkerAndHealth_C|GetHealthBar _aswbp_enemy_marker_and_health) (/ (Variables|Default|GetHealth) (Variables|Default|GetMaxHealth)))
          (Utilities|FlowControl|Sequence
            (:then_0
              (Utilities|FlowControl|DoOnce false :!label _label
                (:Completed
                  (Default|ShowHealthAnim _aswbp_enemy_marker_and_health true))))
            (:then_1
              (Utilities|FlowControl|RetriggerableDelay 5.0)
              (Default|ShowHealthAnim _aswbp_enemy_marker_and_health false)
              (goto _label Reset))))))
    (:then_1
      (bind _aswbp_hud_panels_scanner_main (Utilities|Casting|CastToWBP_HUD_Panels_ScannerMain (UserInterface|GetWidget (Variables|/Game/UltimateSpaceGameKit/Blueprints/BP_PlayerShipdasda.BP_PlayerShipdasda_C|GetCockpitPanel_Scanner (Variables|Default|GetPlayerRef)))))
      (Default|PlayEnemyHitAnim _aswbp_hud_panels_scanner_main))))

(event Game|Damage|EventAnyDamage
  (params (Damage :type Float%20%28single-precision%29) (DamageType :type Damage%20Type%20Object%20Reference) (InstigatedBy :type Controller%20Object%20Reference) (DamageCauser :type Actor%20Object%20Reference))
  (bind _returnvalue (Transformation|GetActorLocation))
  ;[0 0 0] Handle taking damage and death
  (CallFunction|PlayerHitsTargetFeedback)
  (Utilities|FlowControl|Sequence
    (:then_0
      (Utilities|FlowControl|DoOnce false
        (:Completed
          (CallFunction|ChooseBehavior))))
    (:then_1
      (bind _output_get (Variables|Default|SetHealth (- (Variables|Default|GetHealth) Damage)))
      (if (<= _output_get 0.0)
        (Variables|Default|SetIsAlive false)
        (Effects|SpawnEmitteratLocation "/Game/UltimateSpaceGameKit/Particles/PS_EnemyExplosion.PS_EnemyExplosion" (Transformation|GetActorLocation) (Math|Rotator|FindLookatRotation _returnvalue (+ _returnvalue (* (Variables|/Script/Engine.MovementComponent|GetVelocity (Variables|Default|GetFloatingPawnMovement)) 1e+03))))
        (Development|SetHiddeninGame (Variables|Default|GetPS_DistantEnemy) true false)
        (Utilities|FlowControl|Delay (Math|Random|RandomFloatinRange 0.0 2.0))
        (Effects|SpawnEmitteratLocation "/Game/UltimateSpaceGameKit/Particles/PS_EnemyExplosion.PS_EnemyExplosion" (Transformation|GetActorLocation) "0, 0, 0" "4.000000,4.000000,4.000000")
        (Class|NiagaraComponent|SetPaused (Variables|Default|GetNS_RibbonTrail1) true)
        (Variables|/Script/Engine.FloatingPawnMovement|SetMaxSpeed (Variables|Default|GetFloatingPawnMovement) 0.0)
        (Rendering|SetVisibility (Variables|Default|GetSphere) false false)
        (Camera|PlayWorldCameraShake "/Game/UltimateSpaceGameKit/Blueprints/CameraShakes/CS_EnemyExplosionShake.CS_EnemyExplosionShake_C" (Transformation|GetWorldLocation (Variables|Default|GetSphere)) 5e+03 5e+04)
        (Utilities|FlowControl|Delay 3.0)
        (Actor|DestroyActor)))))

(event EventTick
  (params (DeltaSeconds :type Float%20%28single-precision%29))
  (bind _returnvalue (Transformation|GetActorLocation))
  (bind _sphere (Variables|Default|GetSphere))
  (bind _returnvalue_2 (Transformation|GetWorldLocation _sphere))
  ;[0 0 0] tick, avoidance and execute behaviors
  (Utilities|IsValid (Variables|Default|GetPlayerRef)
    (:Is%20Valid
      (CallFunction|ExecuteBehaviour)
      (CallFunction|LeadTargeting)
      (Transformation|SetWorldRotation _sphere (Math|Interpolation|RInterpTo (Transformation|GetWorldRotation _sphere) (Math|Rotator|FindLookatRotation _returnvalue_2 (+ _returnvalue_2 (* (Variables|/Script/Engine.MovementComponent|GetVelocity (Variables|Default|GetFloatingPawnMovement)) 1e+03))) (Utilities|Time|GetWorldDeltaSeconds) 3.0) false false)
      (bind _outhits (Collision|MultiSphereTraceByChannel _returnvalue (+ _returnvalue "10.000000, 0, 0") 1e+03 "TraceTypeQuery1" false 0 "None"))
      (for _array_element _outhits
        (if (.bBlockingHit (Collision|BreakHitResult _array_element))
          (Transformation|SetActorRotation (Math|Rotator|Lerp(Rotator) (Transformation|GetActorRotation) (Math|Conversions|RotationFromXVector (* (.Normal (Collision|BreakHitResult _array_element)) 1e+02)) 0.05)))))))

(event EventBeginPlay
  ;[1 1 1] initialize
  (Variables|Default|SetMaxHealth (Variables|Default|GetHealth))
  (Pawn|SpawnDefaultController)
  (Variables|Default|SetStartingLocation (Transformation|GetActorLocation))
  (CallFunction|CheckforTarget)
  (Utilities|Time|SetTimerbyEvent (EventDispatchers|CreateEvent :!event DisplayUIMarker) (Math|Random|RandomFloatinRange 0.5 1.0) true)
  (Utilities|Time|SetTimerbyEvent (EventDispatchers|CreateEvent :!event Custom|DistanceRelevancy) 1.0 true))

(fn ConstructionScript)

(fn IsTargetWithinAngle
  (params (enemyTarget :type Actor%20Object%20Reference) (ConeAngle :type Float%20%28double-precision%29))
  (return (< (Class|KismetMathLibrary|DegAcos (Math|Vector|DotProduct (Math|Vector|GetForwardVector (Variables|Default|GetSphere)) (Math|Vector|GetUnitDirection(Vector) (Transformation|GetActorLocation) (Transformation|GetActorLocation enemyTarget)))) ConeAngle)))

(fn LeadTargeting
  (LocalVariables|SetRelativePosition (- (Transformation|GetActorLocation (Variables|Default|GetPlayerRef)) (Transformation|GetActorLocation)))
  (Variables|/Script/Engine.SpringArmComponent|SetTargetArmLength (Variables|Default|GetSpringArm) (* (Math|Vector|VectorLength (* (Variables|/Script/Engine.MovementComponent|GetVelocity (Variables|Default|GetFloatingPawnMovement)) (/ (Math|Vector|VectorLength (LocalVariables|GetRelativePosition)) (LocalVariables|GetBulletSpeed)))) -1.0)))

(fn DisplayUIMarker
  (Utilities|IsValid (Variables|Default|GetWidget_MarkerAndHealth)
    (:Is%20Valid
      (Utilities|IsValid (Variables|Default|GetPlayerRef)
        (:Is%20Valid
          (if (Variables|Default|GetIsAlive)
            (Rendering|SetVisibility (Variables|Default|GetWidget_MarkerAndHealth) (< (Math|Vector|VectorLength (- (Transformation|GetActorLocation) (Transformation|GetActorLocation (Game|Player|GetPlayerPawn 0)))) 2e+05) false)
            (else
              (Rendering|SetVisibility (Variables|Default|GetWidget_MarkerAndHealth) false false))))))))