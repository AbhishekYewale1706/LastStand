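; Laser projectile Blueprint that explodes on hit, dealing full radial damage credited to its source weapon, then destroys itself.
; On spawn, collision is off for a brief moment before enabling, and its point light is removed about half a second later.
; Each tick the collision sphere eases toward a maximum radius, a hidden aim assist that makes distant enemies easier and more satisfying to hit.
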(event EventBeginPlay
  (bind _pointlight (Variables|Default|GetPointLight))
  ;[1 1 1] Initialize Projectile
  (Collision|SetCollisionEnabled (Variables|Default|GetSphere) "NoCollision")
  (Utilities|FlowControl|Delay 0.01)
  (Collision|SetCollisionEnabled (Variables|Default|GetSphere) "QueryAndPhysics")
  (Utilities|FlowControl|Delay 0.5)
  (Utilities|IsValid _pointlight
    (:Is%20Valid
      (Components|DestroyComponent _pointlight))))

(event EventTick
  (params (DeltaSeconds :type Float%20%28single-precision%29))
  (bind _sphere (Variables|Default|GetSphere))
  ;[1 1 1] secret gameplay mechanic: we increase the collision radius of each projectile over time, so it feels satisfying to hit enemies that are far away
  (Components|Sphere|SetSphereRadius _sphere (Math|Interpolation|FInterpTo (Variables|/Script/Engine.SphereComponent|GetSphereRadius _sphere) (Variables|Default|GetMaxProjectileRadius) (Utilities|Time|GetWorldDeltaSeconds) 1.0) true))

(event Collision|EventHit
  (params (MyComp :type Primitive%20Component%20Object%20Reference) (Other :type Actor%20Object%20Reference) (OtherComp :type Primitive%20Component%20Object%20Reference) (bSelfMoved :type Boolean) (HitLocation :type Vector :default "0, 0, 0") (HitNormal :type Vector :default "0, 0, 0") (NormalImpulse :type Vector :default "0, 0, 0") (Hit :type Hit%20Result%20Structure%20%28by%20ref%29))
  ;[1 1 1] Play effect, deal damage and destroy actor
  (Effects|SpawnEmitteratLocation "/Game/UltimateSpaceGameKit/Particles/PS_BlasterExplosion.PS_BlasterExplosion" HitLocation)
  (Game|Damage|ApplyRadialDamage (Variables|Default|GetDamage) HitLocation 1e+03 0 0 (Variables|Default|GetSourceActor%28Weapon%29) 0 true "ECC_Visibility")
  (Actor|DestroyActor))

(fn ConstructionScript)