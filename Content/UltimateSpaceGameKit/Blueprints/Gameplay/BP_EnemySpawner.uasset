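; Enemy spawner actor that produces a short burst of enemies around itself at the start of play.
; BeginPlay caches the player ship and runs a fast looping timer, presumably driving SpawnEnemy, then pauses it after a few seconds.
; SpawnEnemy prunes invalid entries from its tracked array and, while under the concurrent cap, spawns the configured class at a random offset.
; Each spawned BP_GenericEnemy receives the player reference and joins the array.
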(event Custom|SpawnEnemy
  (for _array_element (Variables|Default|GetSpawnedEnemies)
    (Utilities|IsValid _array_element
      (:Is%20Not%20Valid
        (Utilities|Array|RemoveItem (Variables|Default|GetSpawnedEnemies) _array_element))))
  (if (< (Utilities|Array|Length (Variables|Default|GetSpawnedEnemies)) (Variables|Default|GetMaxConcurrentEnemies))
    (bind _returnvalue (Game|SpawnActorfromClass (Variables|Default|GetEnemyToSpawn) (Math|Transform|MakeTransform (+ (Transformation|GetActorLocation) (Math|Vector|MakeVector (Math|Random|RandomFloatinRange -1e+04 1e+04) (Math|Random|RandomFloatinRange -1e+04 1e+04) (Math|Random|RandomFloatinRange -1e+04 1e+04))) (Transformation|GetActorRotation) "1.000000,1.000000,1.000000") "Undefined" "SelectDefaultAtRuntime" 0 0))
    (bind _asbp_generic_enemy (Utilities|Casting|CastToBP_GenericEnemy _returnvalue))
    (Variables|/Game/UltimateSpaceGameKit/Blueprints/BP_GenericEnemy.BP_GenericEnemy_C|SetPlayerRef _asbp_generic_enemy (Variables|Default|GetAs%20BP%20Player%20Ship))
    (Utilities|Array|Add (Variables|Default|GetSpawnedEnemies) _asbp_generic_enemy)))

(event EventBeginPlay
  (bind _returnvalue (Utilities|Time|SetTimerbyEvent (EventDispatchers|CreateEvent :!event Custom|SpawnEnemy) 0.2 true))
  (Variables|Default|SetSpawningTimer _returnvalue)
  (bind _asbp_player_ship (Utilities|Casting|CastToBP_PlayerShipdasda (Game|Player|GetPlayerPawn 0)))
  (Variables|Default|SetAs%20BP%20Player%20Ship _asbp_player_ship)
  (Utilities|FlowControl|Delay 3.0)
  (Utilities|Time|PauseTimerbyHandle (Variables|Default|GetSpawningTimer)))

(event Collision|EventActorBeginOverlap
  (params (OtherActor :type Actor%20Object%20Reference)))

(event EventTick
  (params (DeltaSeconds :type Float%20%28single-precision%29)))

(fn ConstructionScript)