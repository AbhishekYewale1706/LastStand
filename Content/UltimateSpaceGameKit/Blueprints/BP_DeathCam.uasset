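; BP_DeathCam is a cinematic camera actor on a spring arm, named as the camera for the player's death.
; On BeginPlay it gives the spring arm a random pitch and yaw for a varied viewing angle.
; Each Tick, while a player pawn exists, it turns the CineCamera toward that pawn, sets focus tracking on it and slowly interpolates the focal length toward a long telephoto zoom.
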(event EventBeginPlay
  (Transformation|SetRelativeRotation (Variables|Default|GetSpringArm) (Math|Rotator|MakeRotator 0.0 (Math|Random|RandomFloatinRange -9e+01 9e+01) (Math|Random|RandomFloatinRange -1.8e+02 1.8e+02)) false false))

(event Collision|EventActorBeginOverlap
  (params (OtherActor :type Actor%20Object%20Reference)))

(event EventTick
  (params (DeltaSeconds :type Float%20%28single-precision%29))
  (bind _returnvalue (Game|Player|GetPlayerPawn 0))
  (bind _cinecamera (Variables|Default|GetCineCamera))
  (bind _cinecamera_2 (Variables|Default|GetCineCamera))
  (Utilities|IsValid (Game|Player|GetPlayerPawn 0)
    (:Is%20Valid
      (Transformation|SetWorldRotation _cinecamera (Math|Rotator|FindLookatRotation (Transformation|GetWorldLocation (Variables|Default|GetCineCamera)) (Transformation|GetActorLocation _returnvalue)) false false)
      (Variables|/Script/CinematicCamera.CineCameraComponent|SetFocusSettings _cinecamera (Utilities|Struct|MakeCameraFocusSettings "Tracking" 1e+05 (Utilities|Struct|MakeCameraTrackingFocusSettings (Utilities|ResolveSoftReference _returnvalue) "0.000000,0.000000,0.000000" false) false 8.0 0.0))
      (Variables|/Script/CinematicCamera.CineCameraComponent|SetCurrentFocalLength _cinecamera_2 (Math|Interpolation|FInterpTo (Variables|/Script/CinematicCamera.CineCameraComponent|GetCurrentFocalLength _cinecamera_2) 8e+02 (Utilities|Time|GetWorldDeltaSeconds) 0.25)))))

(fn ConstructionScript)