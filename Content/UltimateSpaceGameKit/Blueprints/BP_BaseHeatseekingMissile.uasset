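; Base heat-seeking missile for the space game, which explodes with radial damage on reaching its homing target or timing out.
; The sphere overlap ignores everything except the ProjectileMovement homing target component, which this Blueprint does not set itself.
; A hit applies a small damage pulse at the target, then a heavy one after a zero-length delay.
; An untriggered missile self-detonates at its own location after a fixed delay from BeginPlay.
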(event OnComponentBeginOverlap(Sphere)
  (params (OverlappedComponent :type Primitive%20Component%20Object%20Reference) (OtherActor :type Actor%20Object%20Reference) (OtherComp :type Primitive%20Component%20Object%20Reference) (OtherBodyIndex :type Integer) (bFromSweep :type Boolean) (SweepResult :type Hit%20Result%20Structure%20%28by%20ref%29))
  (bind _projectilemovement (Variables|Default|GetProjectileMovement))
  (bind _homingtargetcomponent (Variables|/Script/Engine.ProjectileMovementComponent|GetHomingTargetComponent _projectilemovement))
  (bind _returnvalue (Transformation|GetWorldLocation _homingtargetcomponent))
  (if (== OtherComp _homingtargetcomponent)
    (Effects|SpawnEmitteratLocation "/Game/UltimateSpaceGameKit/Particles/PS_EnemyExplosion.PS_EnemyExplosion" _returnvalue "0, 0, 0" "4.000000,4.000000,4.000000")
    (Game|Damage|ApplyRadialDamage 5.0 _returnvalue 2e+03 0 0 0 0 true "ECC_Pawn")
    (Utilities|FlowControl|Delay 0.0)
    (Game|Damage|ApplyRadialDamage 6e+02 _returnvalue 2e+03 0 0 0 0 true "ECC_Pawn")
    (Actor|DestroyActor)))

(event EventBeginPlay
  (bind _returnvalue (Transformation|GetActorLocation))
  (Utilities|FlowControl|Delay 8.0)
  (Effects|SpawnEmitteratLocation "/Game/UltimateSpaceGameKit/Particles/PS_EnemyExplosion.PS_EnemyExplosion" _returnvalue "0, 0, 0" "4.000000,4.000000,4.000000")
  (Game|Damage|ApplyRadialDamage 5e+02 _returnvalue 2e+03 0 0 0 0 true "ECC_Visibility")
  (Actor|DestroyActor))

(fn ConstructionScript)