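; Enemy actor that homes in on the player, fires lasers, and explodes on contact to deal damage.
; Tick moves it toward the player while spinning until the sight sphere detects them, then it stops and turns to face them.
; A DoOnce-gated looping timer alternates left and right bullets via FlipFlop until sight is lost.
; Damage updates a healthbar widget; death, checked before subtraction, calls EnemyDeath and destroys it.
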(event OnComponentBeginOverlap(Sphere)
  (params (OverlappedComponent :type Primitive%20Component%20Object%20Reference) (OtherActor :type Actor%20Object%20Reference) (OtherComp :type Primitive%20Component%20Object%20Reference) (OtherBodyIndex :type Integer) (bFromSweep :type Boolean) (SweepResult :type Hit%20Result%20Structure%20%28by%20ref%29))
  ;[0.15 0.15 0.15 0.5] Destory /Attack the player if in range
  (if (== OtherActor (Game|Player|GetPlayerPawn 0))
    (Game|Damage|ApplyDamage OtherActor 1e+01 0 0)
    (Effects|SpawnEmitteratLocation "/Game/UltimateSpaceGameKit/Particles/PS_EnemyExplosion.PS_EnemyExplosion" (Transformation|GetActorLocation))
    (Default|CallEnemyDeath)
    (Actor|DestroyActor)))

(event OnComponentBeginOverlap(SpherePlayerSee)
  (params (OverlappedComponent :type Primitive%20Component%20Object%20Reference) (OtherActor :type Actor%20Object%20Reference) (OtherComp :type Primitive%20Component%20Object%20Reference) (OtherBodyIndex :type Integer) (bFromSweep :type Boolean) (SweepResult :type Hit%20Result%20Structure%20%28by%20ref%29))
  ;[0.15 0.15 0.15 0.5] See the player
  (if (== OtherActor (Game|Player|GetPlayerPawn 0))
    (Variables|Default|SetbCanSeePlayer true)))

(event OnComponentEndOverlap(SpherePlayerSee)
  (params (OverlappedComponent :type Primitive%20Component%20Object%20Reference) (OtherActor :type Actor%20Object%20Reference) (OtherComp :type Primitive%20Component%20Object%20Reference) (OtherBodyIndex :type Integer))
  ;[0.15 0.15 0.15 0.5] See the player
  (if (== OtherActor (Game|Player|GetPlayerPawn 0))
    (Variables|Default|SetbCanSeePlayer false)
    (Utilities|Time|ClearandInvalidateTimerbyHandle (Variables|Default|GetStopShooting))
    (CallFunction|ResetFire)))

(event Custom|StartShooting
  ;[0.15 0.15 0.15 0.5] Frie
  (Utilities|FlowControl|FlipFlop
    (:A
      (CallFunction|SpawnBulletL))
    (:B
      (CallFunction|SpawnBulletR))))

(event Custom|Frie
  ;[0.15 0.15 0.15 0.5] Frie
  (bind _returnvalue (Utilities|Time|SetTimerbyEvent (delegate Custom|StartShooting) 0.8 true))
  (Variables|Default|SetStopShooting _returnvalue))

(event Custom|ResetFire
  ;[0.15 0.15 0.15 0.5] Move to player
  (Utilities|FlowControl|DoOnce false) ; enters at Reset
)

(event EventTick
  (params (DeltaSeconds :type Float%20%28single-precision%29))
  (bind _rotatingmovement (Variables|Default|GetRotatingMovement))
  ;[0.15 0.15 0.15 0.5] Move to player
  (if (Variables|Default|GetbCanSeePlayer)
    (CallFunction|LookatPlayer DeltaSeconds)
    (Variables|/Script/Engine.RotatingMovementComponent|SetRotationRate _rotatingmovement "0, 0, 0")
    (Utilities|FlowControl|DoOnce false
      (:Completed
        (CallFunction|Frie)))
    (else
      (CallFunction|MovetoPlayer DeltaSeconds)
      (Variables|/Script/Engine.RotatingMovementComponent|SetRotationRate _rotatingmovement "0.000000,180.000000,0.000000"))))

(event Game|Damage|EventAnyDamage
  (params (Damage :type Float%20%28single-precision%29) (DamageType :type Damage%20Type%20Object%20Reference) (InstigatedBy :type Controller%20Object%20Reference) (DamageCauser :type Actor%20Object%20Reference))
  ;[0.15 0.15 0.15 0.5] Health System
  (if (<= (Variables|Default|GetHealth) 0.0)
    (Effects|SpawnEmitteratLocation "/Game/UltimateSpaceGameKit/Particles/PS_EnemyExplosion.PS_EnemyExplosion" (Transformation|GetActorLocation))
    (Default|CallEnemyDeath)
    (Actor|DestroyActor)
    (else
      (Variables|Default|SetHealth (- (Variables|Default|GetHealth) Damage))
      (bind _aswb_healthbar (Utilities|Casting|CastToWB_Healthbar (UserInterface|GetUserWidgetObject (Variables|Default|GetWidget))))
      (Progress|SetPercent (Variables|/Game/_Main/Blueprints/UI/WB_Healthbar.WB_Healthbar_C|GetHealtbar _aswb_healthbar) (/ (Variables|Default|GetHealth) 1e+02)))))

(fn ConstructionScript)

(fn MovetoPlayer
  (params (DeltaTime :type Float%20%28single-precision%29))
  (Transformation|SetActorLocation (Math|Interpolation|VInterptoConstant (Transformation|GetActorLocation) (Transformation|GetActorLocation (Game|Player|GetPlayerPawn 0)) DeltaTime (Variables|Default|GetInterp%20Speed)) false false))

(fn LookatPlayer
  (params (DeltaTime :type Float%20%28single-precision%29))
  (Transformation|SetActorRotation (Math|Interpolation|RInterpTo (Transformation|GetActorRotation) (Math|Rotator|FindLookatRotation (Transformation|GetActorLocation) (Transformation|GetActorLocation (Game|Player|GetPlayerPawn 0))) DeltaTime 3.0)))

(fn SpawnBulletL
  (bind _arrow (Variables|Default|GetArrow))
  (bind _returnvalue (Transformation|GetWorldTransform _arrow))
  (Game|SpawnActorfromClass "/Game/_Main/Blueprints/Projectile/BP_Bullet.BP_Bullet_C" (Math|Transform|MakeTransform (.location _returnvalue) (.rotation _returnvalue) (.scale _returnvalue)) "AlwaysSpawn" "OverrideRootScale" self false self)
  (Camera|PlayWorldCameraShake "/Game/UltimateSpaceGameKit/Blueprints/CameraShakes/CS_LaserShotCameraShake.CS_LaserShotCameraShake_C" (.location _returnvalue) 1e+01 6e+03)
  (Effects|SpawnEmitterAttached "/Game/UltimateSpaceGameKit/Particles/PS_BlasterFire.PS_BlasterFire" (Variables|Default|GetArrow) "None" "0, 0, 0" "0, 0, 0" "1.000000,1.000000,1.000000" "SnapToTarget"))

(fn SpawnBulletR
  (bind _arrow1 (Variables|Default|GetArrow1))
  (bind _returnvalue (Transformation|GetWorldTransform _arrow1))
  (Game|SpawnActorfromClass "/Game/_Main/Blueprints/Projectile/BP_Bullet.BP_Bullet_C" (Math|Transform|MakeTransform (.location _returnvalue) (.rotation _returnvalue) (.scale _returnvalue)) "AlwaysSpawn" "OverrideRootScale" self false self)
  (Camera|PlayWorldCameraShake "/Game/UltimateSpaceGameKit/Blueprints/CameraShakes/CS_LaserShotCameraShake.CS_LaserShotCameraShake_C" (.location _returnvalue) 1e+01 6e+03)
  (Effects|SpawnEmitterAttached "/Game/UltimateSpaceGameKit/Particles/PS_BlasterFire.PS_BlasterFire" (Variables|Default|GetArrow1) "None" "0, 0, 0" "0, 0, 0" "1.000000,1.000000,1.000000" "SnapToTarget"))