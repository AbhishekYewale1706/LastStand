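; Player ship pawn that flies along the control rotation, fires lasers, and owns the gameplay HUD.
; Firing traces from the camera for an aim point, then alternates left and right bullets toward it.
; AnyDamage updates health or triggers explosion, save and game-over screen; Power charges heal through timed negative damage.
; It loads player data through the game instance and has debug keys for self-damage and clearing data.
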(event Custom|Set%20Text%20of%20Gameplay%20Hud
  (params (TotalEnemy :type Text) (Score :type Text))
  (bind _wb_gameplayref (Variables|Default|GetWB_GameplayRef))
  ;[0.02812 0.02812 0.02812 0.5] Gameplay Hud Text
  (Rendering|Components|TextRender|SetText (Variables|/Game/_Main/Blueprints/UI/WB_Gameplay.WB_Gameplay_C|GetEnemy _wb_gameplayref) TotalEnemy)
  (Rendering|Components|TextRender|SetText (Variables|/Game/_Main/Blueprints/UI/WB_Gameplay.WB_Gameplay_C|GetScore _wb_gameplayref) Score))

(event Custom|Heal
  ;[0.01562 0.01562 0.01562 0.5] Power
  (if (>= (Variables|Default|GetHealth) 1e+02)
    (Utilities|Time|ClearandInvalidateTimerbyHandle (Variables|Default|GetHealPowertimer))
    (else
      (Game|Damage|ApplyDamage self -1e+01 0 0))))

(event Input|EnhancedActionEvents|EnhancedInputActionIA_Look
  (params (ActionValue :type Vector%202D%20Structure) (ElapsedSeconds :type Float%20%28double-precision%29) (TriggeredSeconds :type Float%20%28double-precision%29) (InputAction :type Input%20Action%20Object%20Reference :default "/Game/_Main/Input/Action/IA_Look.IA_Look"))
  ;[0.01979 0.01979 0.01979 0.5] Look Around
  (Pawn|Input|AddControllerYawInput (* (.x ActionValue) (Variables|Default|GetSenX)))
  (Pawn|Input|AddControllerPitchInput (* (.y ActionValue) (Variables|Default|GetSenY))))

(event Input|EnhancedActionEvents|EnhancedInputActionIA_Move
  (params (ActionValue :type Vector%202D%20Structure) (ElapsedSeconds :type Float%20%28double-precision%29) (TriggeredSeconds :type Float%20%28double-precision%29) (InputAction :type Input%20Action%20Object%20Reference :default "/Game/_Main/Input/Action/IA_Move.IA_Move"))
  ;[0.02396 0.02396 0.02396 0.5] Movement
  (CallFunction|MoveRightLeft (.x ActionValue))
  (CallFunction|MoveUpDown (.y ActionValue)))

(event Input|EnhancedActionEvents|EnhancedInputActionIA_Fire
  (params (ActionValue :type Boolean) (ElapsedSeconds :type Float%20%28double-precision%29) (TriggeredSeconds :type Float%20%28double-precision%29) (InputAction :type Input%20Action%20Object%20Reference :default "/Game/_Main/Input/Action/IA_Fire.IA_Fire"))
  ;[0.01562 0.01562 0.01562 0.5] Shooting
  (CallFunction|Aim)
  (Utilities|FlowControl|FlipFlop
    (:A
      (CallFunction|SpawnBulletRight))
    (:B
      (CallFunction|SpawnBulletLeft))))

(event Input|EnhancedActionEvents|EnhancedInputActionIA_Power
  (params (ActionValue :type Boolean) (ElapsedSeconds :type Float%20%28double-precision%29) (TriggeredSeconds :type Float%20%28double-precision%29) (InputAction :type Input%20Action%20Object%20Reference :default "/Game/_Main/Input/Action/IA_Power.IA_Power"))
  ;[0.01562 0.01562 0.01562 0.5] Power
  (:Started
    (if (>= (Variables|Default|GetPower) 1)
      (bind _output_get (Variables|Default|SetPower (- (Variables|Default|GetPower) 1)))
      (Rendering|Components|TextRender|SetText (Variables|/Game/_Main/Blueprints/UI/WB_Gameplay.WB_Gameplay_C|Getpower (Variables|Default|GetWB_GameplayRef)) (Utilities|Text|ToText(Integer) _output_get))
      (bind _returnvalue (Utilities|Time|SetTimerbyEvent (delegate Custom|Heal) 0.3 true))
      (Variables|Default|SetHealPowertimer _returnvalue))))

(event EventBeginPlay
  ;[0.00996 0.3031 0.9323 0.5] Beginplay
  (Utilities|FlowControl|Sequence
    (:then_0
      (bind _asbp_game_instance (Utilities|Casting|CastToBP_GameInstance (Game|GetGameInstance)))
      (Variables|Default|SetAs%20BP%20Game%20InstanceRef _asbp_game_instance)
      (Default|LoadPlayerData (Variables|Default|GetAs%20BP%20Game%20InstanceRef)))
    (:then_1
      (bind _asgm_gameplay (Utilities|Casting|CastToGM_Gameplay (Game|GetGameMode)))
      (Variables|Default|SetAs%20GM%20GameplayRef _asgm_gameplay))
    (:then_2
      (bind _returnvalue (UserInterface|CreateWidget "/Game/_Main/Blueprints/UI/WB_Gameplay.WB_Gameplay_C"))
      (bind _output_get (Variables|Default|SetWB_GameplayRef _returnvalue))
      (UserInterface|Viewport|AddtoViewport _output_get 0))
    (:then_3
      (CallFunction|SetTextOfGameplayHud (Utilities|Text|ToText(Integer) (Variables|/Game/_Main/Blueprints/FrameWork/GM_Gameplay.GM_Gameplay_C|GetTotalEnemy (Variables|Default|GetAs%20GM%20GameplayRef))) "00"))))

(event EventTick
  (params (DeltaSeconds :type Float%20%28single-precision%29))
  ;[1 0 0 0.5] Tick
  ;;[0.15 0.15 0.15 0.5] rotating the mesh
  (Transformation|SetWorldRotation (Variables|Default|GetSkeletalMesh) (Pawn|GetControlRotation :!class /Script/Engine.Pawn) false false))

(event Game|Damage|EventAnyDamage
  (params (Damage :type Float%20%28single-precision%29) (DamageType :type Damage%20Type%20Object%20Reference) (InstigatedBy :type Controller%20Object%20Reference) (DamageCauser :type Actor%20Object%20Reference))
  ;[0.02396 0.02396 0.02396 0.5] Health System
  (if (<= (Variables|Default|GetHealth) 1e+01)
    (Effects|SpawnEmitteratLocation "/Game/UltimateSpaceGameKit/Particles/PS_EnemyExplosion.PS_EnemyExplosion" (Transformation|GetActorLocation))
    (Input|DisableInput (Game|GetPlayerController 0))
    (Rendering|SetVisibility (Variables|Default|GetSkeletalMesh) false false)
    (Utilities|FlowControl|Delay 0.2)
    (bind _returnvalue (UserInterface|CreateWidget "/Game/_Main/Blueprints/UI/WB_GameOver.WB_GameOver_C" (Game|GetPlayerController 0)))
    (Rendering|Components|TextRender|SetText (Variables|/Game/_Main/Blueprints/UI/WB_GameOver.WB_GameOver_C|GetHighScoreText _returnvalue) (Utilities|Text|ToText(Integer) (Variables|/Game/_Main/Blueprints/FrameWork/BP_SaveGame.BP_SaveGame_C|GetHighScore (Variables|/Game/_Main/Blueprints/FrameWork/BP_GameInstance.BP_GameInstance_C|GetSaveGameData (Variables|Default|GetAs%20BP%20Game%20InstanceRef)))))
    (Rendering|Components|TextRender|SetText (Variables|/Game/_Main/Blueprints/UI/WB_GameOver.WB_GameOver_C|GetCurrentScoreText _returnvalue) (Utilities|Text|ToText(Integer) (Variables|/Game/_Main/Blueprints/FrameWork/GM_Gameplay.GM_Gameplay_C|GetCurrentScore (Variables|Default|GetAs%20GM%20GameplayRef))))
    (UserInterface|Viewport|AddtoViewport _returnvalue 0)
    (Default|SavePlayerData (Variables|Default|GetAs%20BP%20Game%20InstanceRef))
    (Game|SetGamePaused true)
    (else
      (Variables|Default|SetHealth (Math|Float|Clamp(Float) (- (Variables|Default|GetHealth) Damage) 1.0 1e+02))
      (Progress|SetPercent (Variables|/Game/_Main/Blueprints/UI/WB_Gameplay.WB_Gameplay_C|GetHealthProgressBar (Variables|Default|GetWB_GameplayRef)) (/ (Variables|Default|GetHealth) 1e+02)))))

(event Input|KeyboardEvents|N
  (params (Key :type Key%20Structure :default "None"))
  ;[0.15 0.15 0.15 0.5] Debug
  (:Pressed
    (Default|ClearPlayerData (Variables|Default|GetAs%20BP%20Game%20InstanceRef))))

(event Input|KeyboardEvents|M
  (params (Key :type Key%20Structure :default "None"))
  ;[0.15 0.15 0.15 0.5] Debug
  (:Pressed
    (Game|Damage|ApplyDamage self 2e+01 0 0)))

(fn ConstructionScript)

(fn Aim
  (bind _camera (Variables|Default|GetCamera))
  (bind _returnvalue (Transformation|GetWorldLocation _camera))
  (bind _output_get (Variables|Default|SetHitLocation (+ _returnvalue (* (Math|Vector|GetForwardVector _camera) (Variables|Default|GetFireDistance)))))
  (bind _outhit (Collision|LineTraceByChannel _returnvalue _output_get "TraceTypeQuery1" false 0 "None"))
  (Variables|Default|SetHitLocation (Math|Vector|SelectVector (.ImpactPoint (Collision|BreakHitResult _outhit)) (Variables|Default|GetHitLocation) (.bBlockingHit (Collision|BreakHitResult _outhit)))))

(fn MoveRightLeft
  (params (B :type Float%20%28double-precision%29))
  (Class|PawnMovementComponent|AddInputVector (Variables|Default|GetFloatingPawnMovement) (* (Math|Vector|GetRightVector (Pawn|GetControlRotation :!class /Script/Engine.Pawn)) B) false))

(fn MoveUpDown
  (params (B :type Float%20%28double-precision%29))
  (Class|PawnMovementComponent|AddInputVector (Variables|Default|GetFloatingPawnMovement) (* (Math|Vector|GetForwardVector (Pawn|GetControlRotation :!class /Script/Engine.Pawn)) B) false))

(fn SpawnBulletRight
  (bind _weaponsr (Variables|Default|GetWeaponsR))
  (bind _returnvalue (Transformation|GetWorldTransform _weaponsr))
  (Game|SpawnActorfromClass "/Game/_Main/Blueprints/Projectile/BP_Bullet.BP_Bullet_C" (Math|Transform|MakeTransform (.location _returnvalue) (Math|Rotator|FindLookatRotation (.location _returnvalue) (Variables|Default|GetHitLocation)) "1.000000,1.000000,1.000000") "AlwaysSpawn" "OverrideRootScale" self true self)
  (Camera|PlayWorldCameraShake "/Game/UltimateSpaceGameKit/Blueprints/CameraShakes/CS_LaserShotCameraShake.CS_LaserShotCameraShake_C" (.location _returnvalue) 1e+01 6e+03)
  (Effects|SpawnEmitterAttached "/Game/UltimateSpaceGameKit/Particles/PS_BlasterFire.PS_BlasterFire" (Variables|Default|GetWeaponsR) "None" "0, 0, 0" "0, 0, 0" "1.000000,1.000000,1.000000" "SnapToTarget"))

(fn SpawnBulletLeft
  (bind _weaponsl (Variables|Default|GetWeaponsL))
  (bind _returnvalue (Transformation|GetWorldTransform _weaponsl))
  (bind _returnvalue_2 (Game|SpawnActorfromClass "/Game/_Main/Blueprints/Projectile/BP_Bullet.BP_Bullet_C" (Math|Transform|MakeTransform (.location _returnvalue) (Math|Rotator|FindLookatRotation (.location _returnvalue) (Variables|Default|GetHitLocation)) "1.000000,1.000000,1.000000") "AlwaysSpawn" "OverrideRootScale" self true self))
  (Collision|IgnoreActorwhenMoving (Variables|/Game/_Main/Blueprints/Projectile/BP_Bullet.BP_Bullet_C|GetBox _returnvalue_2) _returnvalue_2 true)
  (Camera|PlayWorldCameraShake "/Game/UltimateSpaceGameKit/Blueprints/CameraShakes/CS_LaserShotCameraShake.CS_LaserShotCameraShake_C" (.location _returnvalue) 1e+01 6e+03)
  (Effects|SpawnEmitterAttached "/Game/UltimateSpaceGameKit/Particles/PS_BlasterFire.PS_BlasterFire" (Variables|Default|GetWeaponsL) "None" "0, 0, 0" "0, 0, 0" "1.000000,1.000000,1.000000" "SnapToTarget"))