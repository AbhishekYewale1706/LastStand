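; BP_Enemy_1 is a kamikaze enemy that homes in on the player and explodes on contact.
; Tick moves it toward the player pawn at constant speed without sweeping, and its sphere overlap deals damage to the player.
; Incoming damage lowers Health and updates a widget health bar, with death checked before subtraction, so a further hit finishes it.
; Both death paths spawn an explosion, fire the EnemyDeath dispatcher and destroy the actor.
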(event OnComponentBeginOverlap(Sphere)
  (params (OverlappedComponent :type Primitive%20Component%20Object%20Reference) (OtherActor :type Actor%20Object%20Reference) (OtherComp :type Primitive%20Component%20Object%20Reference) (OtherBodyIndex :type Integer) (bFromSweep :type Boolean) (SweepResult :type Hit%20Result%20Structure%20%28by%20ref%29))
  ;[0.15 0.15 0.15 0.5] Destory /Attack the player if in range
  (if (== OtherActor (Game|Player|GetPlayerPawn 0))
    (Game|Damage|ApplyDamage OtherActor 2e+01 0 0)
    (Effects|SpawnEmitteratLocation "/Game/UltimateSpaceGameKit/Particles/PS_EnemyExplosion.PS_EnemyExplosion" (Transformation|GetActorLocation))
    (Default|CallEnemyDeath)
    (Actor|DestroyActor)))

(event EventTick
  (params (DeltaSeconds :type Float%20%28single-precision%29))
  ;[0.15 0.15 0.15 0.5] Move to player
  (Transformation|SetActorLocation (Math|Interpolation|VInterptoConstant (Transformation|GetActorLocation) (Transformation|GetActorLocation (Game|Player|GetPlayerPawn 0)) DeltaSeconds (Variables|Default|GetInterp%20Speed)) false false))

(event Game|Damage|EventAnyDamage
  (params (Damage :type Float%20%28single-precision%29) (DamageType :type Damage%20Type%20Object%20Reference) (InstigatedBy :type Controller%20Object%20Reference) (DamageCauser :type Actor%20Object%20Reference))
  ;[0.15 0.15 0.15 0.5] Health System
  (if (<= (Variables|Default|GetHealth) 0.0)
    (Effects|SpawnEmitteratLocation "/Game/UltimateSpaceGameKit/Particles/PS_EnemyExplosion.PS_EnemyExplosion" (Transformation|GetActorLocation))
    (Default|CallEnemyDeath)
    (Actor|DestroyActor)
    (else
      (Variables|Default|SetHealth (- (Variables|Default|GetHealth) Damage))
      (bind _aswb_healthbar (Utilities|Casting|CastToWB_Healthbar (UserInterface|GetUserWidgetObject (Variables|Default|GetWidget))))
      (Progress|SetPercent (Variables|/Game/_Main/Blueprints/UI/WB_Healthbar.WB_Healthbar_C|GetHealtbar _aswb_healthbar) (/ (Variables|Default|GetHealth) 1e+02)))))

(fn ConstructionScript)