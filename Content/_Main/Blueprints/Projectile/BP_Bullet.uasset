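; BP_Bullet is a blaster projectile that damages whatever it hits.
; On spawn its Box ignores the owner when moving and keeps collision off for a brief delay before enabling it.
; A Box hit spawns an explosion at the impact point, applies Damage to the other actor and destroys the bullet.
; The construction script picks the Cylinder's laser material from IsPlayer, distinguishing player shots from others.
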(event OnComponentHit(Box)
  (params (HitComponent :type Primitive%20Component%20Object%20Reference) (OtherActor :type Actor%20Object%20Reference) (OtherComp :type Primitive%20Component%20Object%20Reference) (NormalImpulse :type Vector :default "0, 0, 0") (Hit :type Hit%20Result%20Structure%20%28by%20ref%29))
  ;[0.15 0.15 0.15 0.5] Hit
  (Effects|SpawnEmitteratLocation "/Game/UltimateSpaceGameKit/Particles/PS_BlasterExplosion.PS_BlasterExplosion" (.ImpactPoint (Collision|BreakHitResult Hit)))
  (Game|Damage|ApplyDamage OtherActor (Variables|Default|GetDamage) 0 0)
  (Actor|DestroyActor))

(event EventBeginPlay
  (Collision|IgnoreActorwhenMoving (Variables|Default|GetBox) (Components|GetOwner) true)
  (Collision|SetCollisionEnabled (Variables|Default|GetBox) "NoCollision")
  (Utilities|FlowControl|Delay 0.02)
  (Collision|SetCollisionEnabled (Variables|Default|GetBox) "QueryAndPhysics"))

(event Collision|EventActorBeginOverlap
  (params (OtherActor :type Actor%20Object%20Reference)))

(event EventTick
  (params (DeltaSeconds :type Float%20%28single-precision%29)))

(fn ConstructionScript
  (if (Variables|Default|GetbIsPlayer?)
    (Rendering|Material|SetMaterial (Variables|Default|GetCylinder) 0 "/Game/UltimateSpaceGameKit/Materials/M_LaserLight.M_LaserLight")
    (else
      (Rendering|Material|SetMaterial (Variables|Default|GetCylinder) 0 "/Game/UltimateSpaceGameKit/Materials/M_LaserLight1.M_LaserLight1"))))