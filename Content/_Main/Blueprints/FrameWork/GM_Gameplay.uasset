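; Gameplay game mode that tracks enemy kills and score and shows the win screen.
; On BeginPlay it loads player data through the game instance, binds each tagged enemy's death event and sets TotalEnemy from the loop's last index, not the array length.
; Each death decrements the count, then either adds score and updates the player ship's HUD or, at zero, saves and displays current and high scores without awarding points.
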(event Custom|EnemyDeath_Event
  (CallFunction|ReduceEnemyCount))

(event EventBeginPlay
  (Utilities|FlowControl|Sequence
    (:then_0
      (bind _asbp_player_ship (Utilities|Casting|CastToBP_PlayerShip (Game|Player|GetPlayerPawn 0)))
      (Variables|Default|SetAs%20BP%20Player%20Ship _asbp_player_ship)
      (bind _asbp_game_instance (Utilities|Casting|CastToBP_GameInstance (Game|GetGameInstance)))
      (bind _output_get (Variables|Default|SetAs%20BP%20Game%20Instance _asbp_game_instance))
      (Default|LoadPlayerData _output_get))
    (:then_1
      (bind _outactors (Actor|GetAllActorsOfClasswithTag "/Game/_Main/Blueprints/Core/BP_EnemyBase.BP_EnemyBase_C" "Enemy"))
      (for (_array_element _array_index) _outactors
        (bind _asbp_enemy_base (Utilities|Casting|CastToBP_EnemyBase _array_element))
        (EventDispatchers|AssignEnemyDeath _asbp_enemy_base (delegate Custom|EnemyDeath_Event)))
      (Variables|Default|SetTotalEnemy _array_index))))

(event EventTick
  (params (DeltaSeconds :type Float%20%28single-precision%29)))

(fn ConstructionScript)

(fn ReduceEnemyCount
  (bind _as_bp_game_instance (Variables|Default|GetAs%20BP%20Game%20Instance))
  (bind _output_get (Variables|Default|SetTotalEnemy (- (Variables|Default|GetTotalEnemy) 1)))
  (if (<= _output_get 0)
    (bind _returnvalue (UserInterface|CreateWidget "/Game/_Main/Blueprints/UI/WB_GameWin.WB_GameWin_C" (Game|GetPlayerController 0)))
    (Default|SavePlayerData _as_bp_game_instance)
    (Rendering|Components|TextRender|SetText (Variables|/Game/_Main/Blueprints/UI/WB_GameWin.WB_GameWin_C|GetHighScoreText _returnvalue) (Utilities|Text|ToText(Integer) (Variables|/Game/_Main/Blueprints/FrameWork/BP_SaveGame.BP_SaveGame_C|GetHighScore (Variables|/Game/_Main/Blueprints/FrameWork/BP_GameInstance.BP_GameInstance_C|GetSaveGameData _as_bp_game_instance))))
    (Rendering|Components|TextRender|SetText (Variables|/Game/_Main/Blueprints/UI/WB_GameWin.WB_GameWin_C|GetCurrentScoreText _returnvalue) (Utilities|Text|ToText(Integer) (Variables|Default|GetCurrentScore)))
    (UserInterface|Viewport|AddtoViewport _returnvalue 0)
    (else
      (Variables|Default|SetCurrentScore (+ (Variables|Default|GetCurrentScore) 10))
      (Default|SetTextOfGameplayHud (Variables|Default|GetAs%20BP%20Player%20Ship) (Utilities|Text|ToText(Integer) (Variables|Default|GetTotalEnemy)) (Utilities|Text|ToText(Integer) (Variables|Default|GetCurrentScore))))))